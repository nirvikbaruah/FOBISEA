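; PuzzleInput is an interactable trigger actor that opens the puzzle UI when the player presses PuzzleInteract within its collider.
; Begin and end overlap set a WithinCollider flag and show or hide the GameHUD prompt text, without checking which actor overlaps.
; It enables player 0 input on BeginPlay, and a press while flagged calls PuzzleUI on the first ThirdPersonCharacter found by GetAllActorsOfClass.
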(event `self.ReceiveActorBeginOverlap`
  (params (OtherActor :type "Actor Object Reference"))
  ;[1 1 1] Checks if User still within Collider
  (set `self.WithinCollider` true)
  (bind _outactors (`GameplayStatics.GetAllActorsOfClass` "/Game/Blueprints/GameHUD.GameHUD_C"))
  (`/Game/Blueprints/GameHUD.ShowPromptText` (`KismetArrayLibrary.Array_Get` _outactors)))

(event `self.ReceiveBeginPlay`
  ;[1 1 1] Allows user input
  (`self.EnableInput` (`GameplayStatics.GetPlayerController` 0)))

(event `self.ReceiveActorEndOverlap`
  (params (OtherActor :type "Actor Object Reference"))
  ;[1 1 1] Checks if User still within Collider
  (set `self.WithinCollider` false)
  (bind _outactors (`GameplayStatics.GetAllActorsOfClass` "/Game/Blueprints/GameHUD.GameHUD_C"))
  (`/Game/Blueprints/GameHUD.HidePromptText` (`KismetArrayLibrary.Array_Get` _outactors)))

(event `InputAction|PuzzleInteract`
  (params (Key :type "Key Structure" :default "AnyKey"))
  ;[1 1 1] If key pressed then checks if object is visible
  (:`Pressed`
    (if (`self.WithinCollider`)
      (bind _outactors (`GameplayStatics.GetAllActorsOfClass` "/Game/Assets/Models/Character/ThirdPersonBP/Blueprints/ThirdPersonCharacter.ThirdPersonCharacter_C"))
      (`/Game/Assets/Models/Character/ThirdPersonBP/Blueprints/ThirdPersonCharacter.PuzzleUI` (`KismetArrayLibrary.Array_Get` _outactors)))))

(fn `UserConstructionScript`)